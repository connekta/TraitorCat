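; Player controller for the multiplayer lobby that manages the player's lobby UI and handles being kicked.
; It creates the lobby widget with server name, map, mode and slots, then forwards player count and player list updates to it.
; Further events swap the lobby widget for a loading screen, or handle a kick by opening the Menu level and destroying the session.
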(event Custom|AddLobbyWB
  (params (ServerName :type String) (ServerMap :type String) (ServerMode :type String) (ServerSlots :type Integer))
  (Variables|Default|SetbShowMouseCursor true)
  (bind _returnvalue (UserInterface|CreateWidget "/Game/UI/Lobby_WB.Lobby_WB_C" self (Utilities|Text|ToText(String) ServerName) (Utilities|Text|ToText(String) ServerMap) (Utilities|Text|ToText(String) ServerMode) ServerSlots))
  (bind _output_get (Variables|Default|SetLobbyWB _returnvalue))
  (UserInterface|Viewport|AddtoViewport _output_get 1))

(event Custom|LoadingScreen
  (Widget|RemovefromParent (Variables|Default|GetLobbyWB))
  (bind _returnvalue (UserInterface|CreateWidget "/Game/UI/LoadingScreen.LoadingScreen_C" self))
  (UserInterface|Viewport|AddtoViewport _returnvalue 0))

(event Custom|AddPlayer
  (params (Player :type Text) (PlayerIndex :type Integer))
  (Default|AddPlayertoList (Variables|Default|GetLobbyWB) Player PlayerIndex))

(event Custom|ClearPlayerList
  (Default|ClearPlayerList (Variables|Default|GetLobbyWB)))

(event Custom|Kick
  (Game|OpenLevel(byName) "Menu")
  (|DestroySession self))

(event Custom|UpdateNumberOfPlayers
  (params (CurrentPlayers :type Integer))
  (Variables|/Game/UI/Lobby_WB.Lobby_WB_C|SetCurrentPlayers (Variables|Default|GetLobbyWB) CurrentPlayers))

(fn ConstructionScript)