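; Networked hinged door Blueprint that supports both a quick open/close toggle and incremental swinging.
; Quick interact goes from a server event to a multicast, which checks hinge yaw and plays or reverses a timeline lerping between closed and open rotations, starting from the current angle.
; OpenCloseDoor scales its input into a yaw step, clamps it to limits relative to the door frame, and multicasts the hinge's new world rotation.
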(event Custom|OpenCloseDoor
  (params (Hodor :type Float%20%28single-precision%29) (Hodor? :type Boolean))
  (bind _doorframe (Variables|Default|GetDoorFrame))
  (bind _hinge (Variables|Default|Gethinge))
  (bind _returnvalue (Transformation|GetWorldRotation _doorframe))
  (bind _yaw (Math|Rotator|BreakRotator _returnvalue))
  (if Hodor?
    (CallFunction|MulticastOpenClose _hinge (Math|Rotator|MakeRotator 0.0 0.0 (Math|Float|Clamp(Float) (.Yaw (Math|Rotator|BreakRotator (Math|Rotator|CombineRotators (Transformation|GetWorldRotation _hinge) (Math|Rotator|MakeRotator 0.0 0.0 (* Hodor -4.0))))) (+ _yaw (Variables|Default|GetMinOpen)) (+ _yaw (Variables|Default|GetMaxOpen)))))))

(event Custom|Multicast_OpenClose
  (params (Target :type Scene%20Component%20Object%20Reference) (NewRotation :type Rotator))
  (Transformation|SetWorldRotation Target NewRotation false false))

(event Custom|MultiCast_QuickInteract
  (bind _hinge (Variables|Default|Gethinge))
  (bind _relativerotation (Variables|/Script/Engine.SceneComponent|GetRelativeRotation _hinge))
  (if (<= (.yaw (Variables|/Script/Engine.SceneComponent|GetRelativeRotation (Variables|Default|Gethinge))) 15.0)
    (Variables|Default|SetClosedDoor _relativerotation)
    (bind _newtrack_0 (Timeline|Timeline_0 PlayFromStart)
      (:Update
        (Transformation|SetRelativeRotation (Variables|Default|Gethinge) (Math|Rotator|Lerp(Rotator) (Variables|Default|GetClosedDoor) (Variables|Default|GetOpenDoor) _newtrack_0) false false))
      (:Finished
        (Variables|Default|SetOpenDoor "0,90.000000, 0")
        (Variables|Default|SetClosedDoor "0, 0, 0")))
    (else
      (Variables|Default|SetOpenDoor _relativerotation)
      (Timeline|Timeline_0 ReverseFromEnd))))

(event Custom|Server_QuickInteract
  (CallFunction|MultiCastQuickInteract))

(fn ConstructionScript)