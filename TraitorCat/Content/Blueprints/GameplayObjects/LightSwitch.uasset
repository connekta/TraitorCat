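; LightSwitch is a gameplay object that turns an array of lights on and off over the network.
; A server event flips the IsActive flag and calls a multicast event, which sets the visibility of each light's LightComponent to match.
; An interact message and a debug print are left unconnected, so nothing in this graph triggers the server event.
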(event Custom|Server_Switch%20Pressed
  (Variables|Default|SetIsActive (not (Variables|Default|GetIsActive)))
  (CallFunction|MulticastSwitchPressed))

(event Custom|Multicast_SwitchPressed
  (for _array_element (Variables|Default|GetLightArray)
    (Rendering|SetVisibility (Variables|/Script/Engine.Light|GetLightComponent _array_element) (Variables|Default|GetIsActive) false)))

(event EventBeginPlay)

(fn ConstructionScript)