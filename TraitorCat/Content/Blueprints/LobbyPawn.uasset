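; Multiplayer lobby pawn that shows each player as a posed character with a name label.
; On BeginPlay it switches the view to the first CineCamera and sends the player name through server and multicast events to a text render that turns each tick.
; The server claims a free LobbySpawnPositions spot, takes its animation and picks a random material.
; RepNotifies apply animation and material, and the color is copied to MyPlayerState after a short delay.
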(event Custom|Server_SetName
  (params (NewVar_0 :type Text))
  ;[1 1 1] Set Player Name over Character
  (Variables|Default|SetPlayerName NewVar_0)
  (CallFunction|MultiCastSetName))

(event Custom|MultiCast_SetName
  ;[1 1 1] Set Player Name over Character
  (Rendering|Components|TextRender|SetText (Variables|Default|GetTextRender) (Variables|Default|GetPlayerName)))

(event Custom|Multicast%20Set%20Occupied
  (params (Target :type Lobby%20Spawn%20Positions%20Object%20Reference))
  ;[1 1 1] Set Spawn Position & Animation
  (Variables|/Game/Blueprints/LobbySpawnPositions.LobbySpawnPositions_C|SetOccupied? Target true)
  (Variables|Default|SetSetPlayerAnimation? true)
  (Utilities|Array|ForEachLoopwithBreak (stale EventBeginPlay _outactors_2)) ; enters at Break
)

(event EventBeginPlay
  (bind _playermaterials (Variables|Default|GetPlayerMaterials))
  (Utilities|FlowControl|Sequence
    (:then_0
      ;[1 1 1] Set Lobby Camera
      (bind _outactors (Actor|GetAllActorsOfClass "/Script/CinematicCamera.CineCameraActor"))
      (Game|Player|SetViewTargetwithBlend (Game|GetPlayerController 0) (Utilities|Array|Get(acopy) _outactors) 0.0 "VTBlend_Linear" 0.0 false))
    (:then_1
      ;[1 1 1] Set Player Name over Character
      (Utilities|FlowControl|Delay 1.0)
      (CallFunction|ServerSetName (Utilities|Text|ToText(String) (Class|AdvancedSessionsLibrary|GetPlayerName (Game|GetPlayerController 0)))))
    (:then_2
      ;[1 1 1] Set Spawn Position & Animation
      (Networking|SwitchHasAuthority
        (:Authority
          (bind _outactors_2 (Actor|GetAllActorsOfClass "/Game/Blueprints/LobbySpawnPositions.LobbySpawnPositions_C"))
          (bind _array_element (Utilities|Array|ForEachLoopwithBreak _outactors_2)
            (:LoopBody
              (if (not (Variables|/Game/Blueprints/LobbySpawnPositions.LobbySpawnPositions_C|GetOccupied? _array_element))
                (Transformation|SetActorTransform (Transformation|GetActorTransform _array_element))
                (Variables|Default|SetAnimDataVar (Variables|/Game/Blueprints/LobbySpawnPositions.LobbySpawnPositions_C|GetAnimationDataVar _array_element))
                (CallFunction|MulticastSetOccupied _array_element)))))))
    (:then_3
      ;[1 1 1] Set PlayerColor (random)
      (Utilities|FlowControl|Sequence
        (:then_0
          (Networking|SwitchHasAuthority ; Set LobbyColors
            (:Authority
              (Variables|Default|SetNewVar_0 (Utilities|Select :Index (Math|Random|RandomIntegerinRange 0 9) :Option%200 (.red _playermaterials) :Option%201 (.bonewhite _playermaterials) :Option%202 (.green _playermaterials) :Option%203 (.blue _playermaterials) :Option%204 (.yellow _playermaterials) :Option%205 (.black _playermaterials) :Option%206 (.brown _playermaterials) :Option%207 (.grey _playermaterials) :Option%208 (.purple _playermaterials) :Option%209 (.white _playermaterials)))
              (Variables|Default|SetPlayerMaterial (Variables|Default|GetNewVar_0)))))
        (:then_1
          (Utilities|FlowControl|Delay 0.2)
          (bind _asmy_player_state (Utilities|Casting|CastToMyPlayerState (Variables|GetPlayerState)))
          (Variables|/Game/Blueprints/MyPlayerState.MyPlayerState_C|SetCosmeticPlayerMaterial _asmy_player_state (Variables|Default|GetNewVar_0)))))))

(event EventTick
  (params (DeltaSeconds :type Float%20%28single-precision%29))
  (bind _textrender (Variables|Default|GetTextRender))
  ;[1 1 1] TextFacingCamera
  (Transformation|SetWorldRotation _textrender (.rotation (Transformation|GetActorTransform (Game|GetPlayerController 0))) false false)
  (Transformation|AddLocalRotation _textrender "0,180.000000, 0" false false))

(fn ConstructionScript)

(fn OnRepNewVar0
  (bind _skeletalmesh (Variables|Default|GetSkeletalMesh))
  (Components|Animation|SetAnimation _skeletalmesh (.animtoplay (Variables|Default|GetAnimDataVar)))
  (Audio|Components|Audio|Play _skeletalmesh true))

(fn OnRepPlayerMaterial
  (Rendering|Material|SetMaterial (Variables|Default|GetSkeletalMesh) 0 (Variables|Default|GetPlayerMaterial)))