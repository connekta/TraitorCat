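; GamePlayerController is a player controller that manages the player's class and health HUD and offers a host-side respawn key.
; Events create a Class_WB widget set from the player status class, push health values into it, or remove all widgets and restore game-only input.
; Pressing I with authority calls RespawnAll on the FirstPersonGameMode.
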(event Custom|UpdatePlayerClass
  (params (PlayerStatus :type Player%20Status%20Structure))
  (bind _returnvalue (UserInterface|CreateWidget "/Game/UI/Class_WB.Class_WB_C" self))
  (bind _output_get (Variables|Default|SetClassWB _returnvalue))
  (UserInterface|Viewport|AddtoViewport _output_get 0)
  (Default|SetClass (Variables|Default|GetClassWB) (.Class (Utilities|Struct|BreakPlayer_Status PlayerStatus))))

(event Custom|UpdatePlayerHealth
  (params (Health :type Text) (HealthFloat :type Float%20%28single-precision%29))
  (bind _classwb (Variables|Default|GetClassWB))
  (Variables|/Game/UI/Class_WB.Class_WB_C|SetHealth _classwb Health)
  (Variables|/Game/UI/Class_WB.Class_WB_C|SetHealthFloat _classwb HealthFloat))

(event Custom|RemoveAllWidgets
  (Input|SetInputModeGameOnly self)
  (Viewport|RemoveAllWidgets))

(event Input|KeyboardEvents|I
  (params (Key :type Key%20Structure))
  (:Pressed
    (if (Ability|HasAuthority)
      (bind _asfirst_person_game_mode (Utilities|Casting|CastToFirstPersonGameMode (Game|GetGameMode)))
      (Default|RespawnAll _asfirst_person_game_mode))))

(fn ConstructionScript)