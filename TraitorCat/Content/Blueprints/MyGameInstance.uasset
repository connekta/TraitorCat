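; Game instance Blueprint that hosts a multiplayer lobby through an advanced session.
; CreateLobby stores the requested server settings, then creates the session with name, map, mode and a LAN flag as extra settings, using the slot count for public connections.
; The method flag also toggles LAN use, and on success the chosen map opens as a listen server.
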(event Custom|CreateLobby
  (params (ServerName :type String) (ServerMap :type String) (ServerSlots :type Integer) (ServerMode :type String) (ServerMethod :type Boolean))
  (Variables|Default|SetServerName ServerName)
  (Variables|Default|SetServerMap ServerMap)
  (Variables|Default|SetServerSlots ServerSlots)
  (Variables|Default|SetServerMode ServerMode)
  (Variables|Default|SetServerMethod ServerMethod)
  (|AdvancedSession (Utilities|Array|MakeArray (Class|AdvancedSessionsLibrary|MakeLiteralSessionPropertyString "NAME" (Variables|Default|GetServerName)) (Class|AdvancedSessionsLibrary|MakeLiteralSessionPropertyString "MAP" (Variables|Default|GetServerMap)) (Class|AdvancedSessionsLibrary|MakeLiteralSessionPropertyString "MODE" (Variables|Default|GetServerMode)) (Class|AdvancedSessionsLibrary|MakeLiteralSessionPropertyBool "LAN" (Variables|Default|GetServerMethod))) (Game|GetPlayerController 0) (Variables|Default|GetServerSlots) 0 (Variables|Default|GetServerMethod) true false true true false false false true
    (:OnSuccess
      (Game|OpenLevel(byName) (Utilities|String|StringToName (Variables|Default|GetServerMap)) true "listen"))))