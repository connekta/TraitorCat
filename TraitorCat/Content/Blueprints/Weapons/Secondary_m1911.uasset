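; Secondary M1911 pistol weapon Blueprint that extends a parent weapon class and leaves firing to the parent.
; On BeginPlay, when owned by a MainCharacter, it sets pistol-specific left-hand IK transforms for hip and aim poses in first and third person.
; It pushes the non-aim transforms into each mesh's Character_AnimBP as left-hand IK targets, while the aim transforms are only stored.
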(event Collision|EventActorBeginOverlap
  (params (OtherActor :type Actor%20Object%20Reference))
  (|CallParentFunction OtherActor) ; This node is disabled and will not be called.\nDrag off pins to build functionality.
)

(event EventTick
  (params (DeltaSeconds :type Float%20%28single-precision%29))
  (|CallParentFunction DeltaSeconds) ; This node is disabled and will not be called.\nDrag off pins to build functionality.
)

(event EventFire
  (|CallParentFunction))

(event EventBeginPlay
  (bind _returnvalue (Components|GetOwner))
  (bind _asmain_character (Utilities|Casting|CastToMainCharacter _returnvalue))
  (|CallParentFunction)
  (Utilities|Casting|CastToMainCharacter (Components|GetOwner)) ; Only do The following if owned by player
  (Utilities|FlowControl|Sequence
    (:then_0
      (Variables|Default|SetFP_LeftHandIK (Math|Transform|MakeTransform "-2.235000,-9.834000,2.715000" "159.057358,84.444298,-4.132879" "1,1,1"))
      (Variables|Default|SetFP_LeftHandAimIK (Math|Transform|MakeTransform "-0.911000,-7.178000,4.654000" "173.271393,80.510124,-6.688824" "1,1,1"))
      (Variables|/Game/Assets/Character/Character_AnimBP.Character_AnimBP_C|SetFirstPerson_LeftHandIKTargetTransform (.AsCharacter%20Anim%20BP (Utilities|Casting|CastToCharacter_AnimBP (Components|SkeletalMesh|GetAnimInstance (Variables|/Game/Blueprints/MainCharacter.MainCharacter_C|GetFirstPersonCharacter _asmain_character)))) (Variables|Default|GetFP_LeftHandIK)))
    (:then_1
      (Variables|Default|Set3P_LeftHandIK (Math|Transform|MakeTransform "-2.437000,-11.473000,2.170000" "156.710464,87.085342,-6.547310" "1,1,1"))
      (Variables|Default|Set3P_LeftHandAimIK (Math|Transform|MakeTransform "-2.691000,-11.432000,2.632000" "156.710419,87.008545,-6.547392" "1,1,1"))
      (Variables|/Game/Assets/Character/Character_AnimBP.Character_AnimBP_C|SetThirdPerson_LeftHandIKTargetTransform (.AsCharacter%20Anim%20BP (Utilities|Casting|CastToCharacter_AnimBP (Components|SkeletalMesh|GetAnimInstance (Variables|/Game/Blueprints/MainCharacter.MainCharacter_C|GetThirdPersonCharacter _asmain_character)))) (Variables|Default|Get3P_LeftHandIK)))))

(fn ConstructionScript
  (|CallParentFunction))