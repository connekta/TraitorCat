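; Base weapon Blueprint providing hitscan firing, owner-based mesh visibility for first/third-person views, and optional server-set physics on spawn.
; Fire spends ammo, line traces from the owner's first-person camera and sends MainCharacter hits to the server for damage.
; The server trusts the reported hit at low ping, but re-traces before applying damage above the ping threshold.
; An explosion emitter at the trace end is multicast through the server; StopFire is empty.
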(event Custom|OwnerNoSee
  ;[1 1 1] Hide/Show ThridPerson Weapon (for First / Third person views)
  (Class|PrimitiveComponent|SetOwnerNoSee (Variables|Default|GetMesh) true))

(event Custom|OwnerOnlySee
  (bind _mesh (Variables|Default|GetMesh))
  ;[1 1 1] Hide/Show ThridPerson Weapon (for First / Third person views)
  (Rendering|SetOnlyOwnerSee _mesh true :!class /Script/Engine.PrimitiveComponent)
  (Rendering|SetCastShadow _mesh false))

(event Custom|Server_VerifyHit
  (params (HitInfo :type Hit%20Result%20Structure) (InstigatorPlayer :type Main%20Character%20Object%20Reference) (HitActor :type Actor%20Object%20Reference))
  ;[1 1 1] Deal Damage
  (if (<= (* (Math|Conversions|ToInteger(Byte) (Variables|/Script/Engine.PlayerState|GetPing (Variables|/Script/Engine.Pawn|GetPlayerState InstigatorPlayer))) 4) 150) ; Ping Over 150 Will have server verify damage
    (Game|Damage|ApplyDamage HitActor (Variables|Default|GetDamage) (Pawn|GetController InstigatorPlayer) self)
    (else
      (bind _hitresult (CallFunction|CalculateShootInformations (Variables|/Game/Blueprints/MainCharacter.MainCharacter_C|GetFirstPersonCamera InstigatorPlayer) InstigatorPlayer))
      (Utilities|Casting|CastToMainCharacter (.HitActor (Collision|BreakHitResult _hitresult))) ; Hit a Player?
      (Game|Damage|ApplyDamage (.HitActor (Collision|BreakHitResult _hitresult)) (Variables|Default|GetDamage) (Pawn|GetController InstigatorPlayer) self))))

(event Custom|Server_SpawnEmitterAtLocation
  (params (Location :type Vector))
  ;[1 1 1] Need to make this only play locally for Instigator and multicast to the rest
  (CallFunction|MultiCastSpawnEmitteratLocation Location))

(event Custom|MultiCast_SpawnEmitterAtLocation
  (params (Location :type Vector))
  ;[1 1 1] Need to make this only play locally for Instigator and multicast to the rest
  (Effects|SpawnEmitteratLocation "/Game/StarterContent/Particles/P_Explosion.P_Explosion" Location "0, 0, 0" "0.500000,0.500000,0.500000"))

(fn ConstructionScript
  (CallFunction|EnablePhysics?))

(fn Fire
  (bind _returnvalue (Components|GetOwner))
  (bind _asmain_character (Utilities|Casting|CastToMainCharacter _returnvalue))
  (Variables|Default|SetCurrentAmmoInMag (- (Variables|Default|GetCurrentAmmoInMag) 1))
  (bind (_hitresult _endlocation) (CallFunction|CalculateShootInformations (Variables|/Game/Blueprints/MainCharacter.MainCharacter_C|GetFirstPersonCamera _asmain_character) _asmain_character))
  (CallFunction|PlayerHit? _hitresult _asmain_character)
  (CallFunction|ServerSpawnEmitteratLocation _endlocation))

(fn EnablePhysics?
  (bind _mesh (Variables|Default|GetMesh))
  (Networking|SwitchHasAuthority
    (:Authority
      (if (Variables|Default|GetEnablePhysicsOnSpawn?)
        (Physics|SetSimulatePhysics _mesh true)
        (else
          (Physics|SetSimulatePhysics _mesh false))))))

(fn StopFire)

(fn CalculateShootInformations
  (params (Camera :type Camera%20Component%20Object%20Reference) (SelfCharacter :type Main%20Character%20Object%20Reference))
  (Utilities|FlowControl|Sequence
    (:then_0
      (LocalVariables|SetLocalCamera Camera))
    (:then_1
      (LocalVariables|SetLocalEndLoc (+ (.location (Transformation|GetWorldTransform (LocalVariables|GetLocalCamera))) (* (Math|Vector|GetForwardVector (.rotation (Transformation|GetWorldTransform (LocalVariables|GetLocalCamera)))) 1e+04)))
      (bind (_outhit _returnvalue) (Collision|LineTraceByChannel (.location (Transformation|GetWorldTransform (LocalVariables|GetLocalCamera))) (+ (.location (Transformation|GetWorldTransform (LocalVariables|GetLocalCamera))) (* (Math|Vector|GetForwardVector (.rotation (Transformation|GetWorldTransform (LocalVariables|GetLocalCamera)))) 1e+04)) "TraceTypeQuery1" false (Utilities|Array|MakeArray SelfCharacter self) "None"))
      (if _returnvalue
        (LocalVariables|SetLocalEndLoc (.ImpactPoint (Collision|BreakHitResult _outhit)))))
    (:then_2
      (if _returnvalue
        (return _outhit (LocalVariables|GetLocalEndLoc))))))

(fn PlayerHit?
  (params (HitResult :type Hit%20Result%20Structure) (Instigator :type Main%20Character%20Object%20Reference))
  (bind _hitactor (Collision|BreakHitResult HitResult))
  (Utilities|Casting|CastToMainCharacter _hitactor) ; Hit a Player?
  (CallFunction|ServerVerifyHit HitResult Instigator _hitactor))